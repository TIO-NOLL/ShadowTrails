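; Game mode for Shadow that sets up the HUD and handles the game clear and game over flows.
; BeginPlay adds near-object and HP widgets, passing an audio component to the latter, and starts wind audio.
; GameClear (with a sound) and GameOver show result widgets, then open Title after a delay.
; Two ungated AnyKey events also open Title; the HP UI events are empty, and some leftover nodes are unwired.
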(event `self.ReceiveBeginPlay`
  (bind _returnvalue (`|CreateWidget` "/Game/Widget/BP/NearObjectWidgetBP.NearObjectWidgetBP_C"))
  (`UserWidget.AddToViewport` _returnvalue 0)
  (bind _returnvalue_2 (`AddComponent|NODE_AddAudioComponent-1`))
  (bind _returnvalue_3 (`|CreateWidget` "/Game/Widget/BP/HPWidgetBP.HPWidgetBP_C" null _returnvalue_2))
  (`UserWidget.AddToViewport` _returnvalue_3 0)
  (`GameplayStatics.PlaySound2D` "/Game/Audio/Wind_Cue.Wind_Cue" 1.0 1.0 0.0 null null))

(event `Key|AnyKey`
  (params (Key :type "Key Structure"))
  ;[1 1 1] クリア時の処理
  (:`Pressed`
    (`GameplayStatics.OpenLevelBySoftObjectPtr` "/Game/title/Title.Title" :!label _label)))

(event `GameClear`
  ;[1 1 1] クリア時の処理
  (`GameplayStatics.PlaySound2D` null 1.0 1.0 0.0 null null)
  (bind _returnvalue (`|CreateWidget` "/Game/GameClear/GameClear_BP.GameClear_BP_C"))
  (`UserWidget.AddToViewport` _returnvalue 0)
  (`KismetSystemLibrary.Delay` 7.0)
  (goto _label))

(event `Key|AnyKey`
  (params (Key :type "Key Structure"))
  ;[1 1 1] ゲームオーバー時の処理
  (:`Pressed`
    (`GameplayStatics.OpenLevelBySoftObjectPtr` "/Game/title/Title.Title" :!label _label_2)))

(event `GameOver`
  ;[1 1 1] ゲームオーバー時の処理
  (bind _returnvalue (`|CreateWidget` "/Game/GameOver/GameOver_BP.GameOver_BP_C"))
  (`UserWidget.AddToViewport` _returnvalue 0)
  (`KismetSystemLibrary.Delay` 5.0)
  (goto _label_2))

(event `create HP UI`)

(event `remove HP UI`)

(fn `UserConstructionScript`)