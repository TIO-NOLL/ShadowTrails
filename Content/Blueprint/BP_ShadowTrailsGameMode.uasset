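; Game mode Blueprint for ShadowTrails that sets up the HUD and runs the clear, game-over and restart flows.
; BeginPlay shows nearby-object, HP and mouse-user widgets, gives the HP widget an audio component, and starts wind audio.
; Game clear opens the Title level after a delay; game over waits out its animation, then respawns the player at the current point.
; Restart, called from C++, resets HP and shows a timed overlay.
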(event `GameClear`
  ;[1 1 1] クリア時の処理
  (`GameplayStatics.PlaySound2D` "/Game/Audio/GameClear.GameClear" 1.0 1.0 0.0 null null)
  (bind _returnvalue (`|CreateWidget` "/Game/GameClear/GameClear_BP.GameClear_BP_C"))
  (`UserWidget.AddToViewport` _returnvalue 0)
  (`KismetSystemLibrary.Delay` 7.0)
  (`GameplayStatics.OpenLevelBySoftObjectPtr` "/Game/title/Title.Title"))

(event `self.ReceiveBeginPlay`
  ;[1 1 1] widgetの作成、表示
  (bind _returnvalue (`|CreateWidget` "/Game/Widget/BP/NearObjectWidgetBP.NearObjectWidgetBP_C"))
  (`UserWidget.AddToViewport` _returnvalue 0)
  (bind _returnvalue_2 (`AddComponent|NODE_AddAudioComponent-0`)) ; damageの音
  (bind _returnvalue_3 (`|CreateWidget` "/Game/Widget/BP/HPWidgetBP.HPWidgetBP_C" null _returnvalue_2))
  (`UserWidget.AddToViewport` _returnvalue_3 0)
  (`GameplayStatics.PlaySound2D` "/Game/Audio/Wind_Cue.Wind_Cue" 1.0 1.0 0.0 null null) ; bgmを流す
  (bind _returnvalue_4 (`|CreateWidget` "/Game/Widget/BP/MouseUserWidgetBP.MouseUserWidgetBP_C"))
  (`UserWidget.AddToViewport` _returnvalue_4 0))

(event `GameOver`
  ;[1 1 1] ゲームオーバー時の処理
  (`KismetSystemLibrary.Delay` 0.5)
  (`GameplayStatics.PlaySound2D` "/Game/Audio/GameOverSound.GameOverSound" 1.0 1.0 0.0 null null)
  (bind _returnvalue (`|CreateWidget` "/Game/GameOver/GameOver_BP.GameOver_BP_C"))
  (`UserWidget.AddToViewport` _returnvalue 0)
  (`KismetSystemLibrary.Delay` (`WidgetAnimation.GetEndTime` (`/Game/GameOver/GameOver_BP.GameOverAnim` _returnvalue)))
  (bind _asbp_player_character (cast `/Game/Blueprint/BP_PlayerCharacter` (`GameplayStatics.GetPlayerCharacter` 0)))
  (`self.RestartPlayerToCurrentPoint` _asbp_player_character)
  (`Widget.RemoveFromParent` _returnvalue))

(event `self.Restart`
  ;[1 1 1] リスタート時の処理(C++上でイベント呼び出し)
  (`/Game/Widget/BP/HPWidgetBP.HPReset` (stale `self.ReceiveBeginPlay` _returnvalue_3))
  (bind _returnvalue (`|CreateWidget` "/Game/GameOver/WBP_Restart.WBP_Restart_C"))
  (`UserWidget.AddToViewport` _returnvalue 0)
  (`KismetSystemLibrary.Delay` (`WidgetAnimation.GetEndTime` (`/Game/GameOver/WBP_Restart.RestatAnim` _returnvalue)))
  (`Widget.RemoveFromParent` _returnvalue))

(event `ResetPlayerHP`
  (`/Game/Widget/BP/HPWidgetBP.HPReset` (stale `self.ReceiveBeginPlay` _returnvalue_3)))

(fn `UserConstructionScript`)